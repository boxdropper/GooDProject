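; BP_StreetLight is a configurable street light actor built around a spot light.
; The construction script picks a light function material from LightStyle for fully on, noticeable flicker or off, then applies the exposed color and intensity.
; Flicker and off states come entirely from light function materials, with no runtime event logic.
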(event EventBeginPlay)

(event Collision|EventActorBeginOverlap
  (params (OtherActor :type Actor%20Object%20Reference)))

(event EventTick
  (params (DeltaSeconds :type Float%20%28single-precision%29)))

(fn ConstructionScript
  (bind _spotlight (Variables|Default|GetSpotLight))
  (Utilities|FlowControl|Sequence
    (:then_0
      (switch Utilities|FlowControl|Switch|SwitchonEnum_StreetLightType (Variables|Default|GetlightStyle)
        (:NewEnumerator0
          (Rendering|Components|Light|SetLightFunctionMaterial _spotlight 0))
        (:NewEnumerator2
          (Rendering|Components|Light|SetLightFunctionMaterial _spotlight "/Game/GooD_Content/Materials/MAT_LightFlicker.MAT_LightFlicker"))
        (:NewEnumerator4
          (Rendering|Components|Light|SetLightFunctionMaterial _spotlight "/Game/GooD_Content/Materials/MAT_LightFlicker_Off.MAT_LightFlicker_Off"))))
    (:then_1
      (Rendering|Components|Light|SetLightColor _spotlight (Variables|Default|GetlightColor) true))
    (:then_2
      (Rendering|Components|Light|SetIntensity _spotlight (Variables|Default|GetlightIntensity)))))